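; Game mode for Mission 03 that manages the mission's on-screen UI.
; On BeginPlay it creates the mission HUD widget for the first player controller and adds it to the viewport.
; Mission failure and completion events show the mission-failed widget and the game-complete menu, respectively.
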(event EventBeginPlay
  (bind _returnvalue (UserInterface|CreateWidget "/Game/HackGameAI/UI/WBP_MissionHUD.WBP_MissionHUD_C" (Game|GetPlayerController 0)))
  (UserInterface|Viewport|AddtoViewport _returnvalue 0))

(event EventTick
  (params (DeltaSeconds :type Float%20%28single-precision%29)))

(event EventOnMissionCompleted
  (params (bIsFinal :type Boolean))
  (bind _returnvalue (UserInterface|CreateWidget "/Game/HackGameAI/UI/WBP_GameCompleteMenu.WBP_GameCompleteMenu_C" (Game|GetPlayerController 0)))
  (UserInterface|Viewport|AddtoViewport _returnvalue 10))

(event EventOnMissionFailed
  (bind _returnvalue (UserInterface|CreateWidget "/Game/HackGameAI/UI/WBP_MissionFailed.WBP_MissionFailed_C" (Game|GetPlayerController 0)))
  (UserInterface|Viewport|AddtoViewport _returnvalue 10))

(fn ConstructionScript)