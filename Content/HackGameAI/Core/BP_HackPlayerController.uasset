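; BP_HackPlayerController is a player controller that shows and hides the pause menu when the game's pause state toggles.
; On pause, OnPauseToggled creates WBP_PauseMenu on first use or reuses the cached widget, adds it to the viewport and gives it UI-only input.
; On unpause it removes the widget if valid and restores Game and UI input mode.
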(event EventBeginPlay)

(event EventTick
  (params (DeltaSeconds :type Float%20%28single-precision%29)))

(event EventOnPauseToggled
  (params (bIsPaused :type Boolean))
  (bind _self self)
  (if bIsPaused
    (Utilities|IsValid (Variables|Default|GetPauseMenuWidget)
      (:Is%20Valid
        (UserInterface|Viewport|AddtoViewport (Variables|Default|GetPauseMenuWidget) 10)
        (Input|SetInputModeUIOnly _self (Variables|Default|GetPauseMenuWidget) "DoNotLock" false))
      (:Is%20Not%20Valid
        (bind _returnvalue (UserInterface|CreateWidget "/Game/HackGameAI/UI/WBP_PauseMenu.WBP_PauseMenu_C" _self))
        (Variables|Default|SetPauseMenuWidget _returnvalue)
        (UserInterface|Viewport|AddtoViewport _returnvalue 10)
        (Input|SetInputModeUIOnly _self _returnvalue "DoNotLock" false)))
    (else
      (Utilities|IsValid (Variables|Default|GetPauseMenuWidget)
        (:Is%20Valid
          (Widget|RemovefromParent (Variables|Default|GetPauseMenuWidget))
          (Input|SetInputModeGameandUI _self 0 "DoNotLock" true false))
        (:Is%20Not%20Valid
          (Input|SetInputModeGameandUI _self 0 "DoNotLock" true false))))))

(fn ConstructionScript)