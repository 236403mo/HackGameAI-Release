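; BP_GateBeam is a mission gate beam that acts as a barrier visual with a glow that switches off on unlock.
; The construction script stretches the mesh along Y from GateLength, keeping a fixed thickness and height.
; OnBarrierUnlocked hides the front, back, top and bottom glow components; the mesh itself is left untouched.
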(event EventBeginPlay)

(event Collision|EventActorBeginOverlap
  (params (OtherActor :type Actor%20Object%20Reference)))

(event EventTick
  (params (DeltaSeconds :type Float%20%28single-precision%29)))

(event EventOnBarrierUnlocked
  (Rendering|SetVisibility (Variables|Default|GetFrontGlow) false false)
  (Rendering|SetVisibility (Variables|Default|GetBackGlow) false false)
  (Rendering|SetVisibility (Variables|Default|GetTopGlow) false false)
  (Rendering|SetVisibility (Variables|Default|GetBottomGlow) false false))

(fn ConstructionScript
  (Transformation|SetRelativeScale3D (Variables|Character|GetMesh) (Math|Vector|MakeVector 0.2 (/ (Variables|Default|GetGateLength) (Math|Float|MakeLiteralFloat 1e+02)) 0.5)))